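; BP_EnemyDummy_2 is a damageable enemy dummy with a billboarded health bar widget.
; Tick updates the bar and HP text, turns the widget toward the camera and hides it while DieDummy is set.
; AnyDamage calls NewDamaged, then plays a hit reaction and sound, or a death animation, kill sound and kill UI on the Genji player at zero HP.
; Any actor overlapping its mesh is destroyed.
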(event OnComponentBeginOverlap(Mesh3P)
  (params (OverlappedComponent :type Primitive%20Component%20Object%20Reference) (OtherActor :type Actor%20Object%20Reference) (OtherComp :type Primitive%20Component%20Object%20Reference) (OtherBodyIndex :type Integer) (bFromSweep :type Boolean) (SweepResult :type Hit%20Result%20Structure%20%28by%20ref%29))
  (Actor|DestroyActor OtherActor))

(event EventBeginPlay
  (bind _asbp_enemy_widget (Utilities|Casting|CastToBP_EnemyWidget (UserInterface|GetWidget (Variables|Default|GetWidget))))
  (bind _asbp_genji_2 (Utilities|Casting|CastToBP_Genji2 (Game|GetPlayerCharacter 0)))
  (Variables|Default|SetAs%20BP%20Genji%202 _asbp_genji_2))

(event Collision|EventActorBeginOverlap
  (params (OtherActor :type Actor%20Object%20Reference)))

(event EventTick
  (params (DeltaSeconds :type Float%20%28single-precision%29))
  (bind _hp_cur (Variables|Default|GetHP_Cur))
  (Progress|SetPercent (Variables|/Game/PKM/Enemy/UI/BP_EnemyWidget.BP_EnemyWidget_C|Getpb_healthBar (stale EventBeginPlay _asbp_enemy_widget)) (/ (Math|Conversions|ToFloat(Integer) _hp_cur) (Math|Conversions|ToFloat(Integer) (Variables|Default|GetHP_Max))))
  (Transformation|SetWorldRotation (Variables|Default|GetWidget) (Math|Rotator|FindLookatRotation (Transformation|GetWorldLocation (Variables|Default|GetWidget)) (Transformation|GetWorldLocation (Variables|/Script/Engine.PlayerCameraManager|GetTransformComponent (Game|GetPlayerCameraManager 0)))) false false)
  (Variables|/Script/UMG.TextBlock|SetText (Variables|/Game/PKM/Enemy/UI/BP_EnemyWidget.BP_EnemyWidget_C|GetCurHP_Text (stale EventBeginPlay _asbp_enemy_widget)) (Utilities|Text|ToText(Integer) _hp_cur))
  (if (Variables|Default|GetbDieDummy)
    (Widget|SetVisibility (stale EventBeginPlay _asbp_enemy_widget) "Hidden")
    (else
      (Widget|SetVisibility (stale EventBeginPlay _asbp_enemy_widget) "Visible"))))

(event Game|Damage|EventAnyDamage
  (params (Damage :type Float%20%28single-precision%29) (DamageType :type Damage%20Type%20Object%20Reference) (InstigatedBy :type Controller%20Object%20Reference) (DamageCauser :type Actor%20Object%20Reference))
  (bind _mesh3p (Variables|Default|GetMesh3P))
  (Class|OValTanCharacter|NewDamaged (Math|Float|Truncate Damage))
  (if (<= (Variables|Default|GetHP_Cur) 0)
    (Default|PlayKilling (Variables|/Game/JJH/blueprint/BP_Genji2.BP_Genji2_C|GetIngame%20UI (Variables|Default|GetAs%20BP%20Genji%202)))
    (Audio|PlaySound2D "/Game/SFX/SFX_UI/SFX_Kill.SFX_Kill" 1.0 1.0 0.0 0 0)
    (Components|Animation|PlayAnimation _mesh3p "/Game/CYS/CYS_Genji/G_Anim/G_Death.G_Death" false)
    (else
      (Components|Animation|PlayAnimation _mesh3p "/Game/CYS/CYS_Genji/G_Anim/G_Locomotion/Crouch_Turn_Left_90.Crouch_Turn_Left_90" false)
      (Audio|PlaySoundatLocation "/Game/SFX/SFX_UI/SFX_HeadShot.SFX_HeadShot" (Transformation|GetWorldLocation _mesh3p) "0, 0, 0" 1.0 1.0 0.0 0 0 0 0))))

(fn ConstructionScript)