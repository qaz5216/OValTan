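; BP_Pyochang_2 is a thrown projectile (pyochang, a shuriken) for the Genji player character, BP_Genji2.
; On BeginPlay it traces forward from the first-person camera, then a timeline lerps it with sweep to the trace's end point, not the impact point.
; Sphere overlaps apply fixed damage, add capped ultimate charge to Genji and update the attack UI, detecting headshots by "Head" in the component name.
; The trace leaves persistent debug lines.
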(event OnComponentBeginOverlap(Sphere)
  (params (OverlappedComponent :type Primitive%20Component%20Object%20Reference) (OtherActor :type Actor%20Object%20Reference) (OtherComp :type Primitive%20Component%20Object%20Reference) (OtherBodyIndex :type Integer) (bFromSweep :type Boolean) (SweepResult :type Hit%20Result%20Structure%20%28by%20ref%29))
  (Game|Damage|ApplyDamage OtherActor 27.0 0 0)
  (bind _asbp_genji_2 (Utilities|Casting|CastToBP_Genji2 (Components|GetOwner)))
  (if (> (+ (Variables|/Script/OValTan.OValTanCharacter|GetGauge_Ultimate_Cur _asbp_genji_2) 2.7) 1e+02)
    (Variables|/Script/OValTan.OValTanCharacter|SetGauge_Ultimate_Cur _asbp_genji_2 1e+02)
    (else
      (Variables|/Script/OValTan.OValTanCharacter|SetGauge_Ultimate_Cur _asbp_genji_2 (+ (Variables|/Script/OValTan.OValTanCharacter|GetGauge_Ultimate_Cur _asbp_genji_2) 2.7))))
  (Default|SetCURUlt (Variables|/Game/JJH/blueprint/BP_Genji2.BP_Genji2_C|GetIngame%20UI _asbp_genji_2))
  (Default|PlayAttack (Variables|/Game/JJH/blueprint/BP_Genji2.BP_Genji2_C|GetIngame%20UI _asbp_genji_2))
  (if (Utilities|String|Contains (Utilities|GetObjectName OtherComp) "Head")
    (Default|AttackHead (Variables|/Game/JJH/blueprint/BP_Genji2.BP_Genji2_C|GetIngame%20UI _asbp_genji_2))))

(event Custom|DashMovement
  (bind _alpha (Timeline|Timeline PlayFromStart)
    (:Update
      (Transformation|SetActorLocation (Math|Vector|Lerp(Vector) (Variables|Default|Getstartlocation) (Variables|Default|GetPyochanglocation) _alpha) true false))))

(event EventBeginPlay
  (bind _asbp_genji_2 (Utilities|Casting|CastToBP_Genji2 (Game|GetPlayerCharacter 0)))
  (bind _outhit (Collision|LineTraceByChannel (Transformation|GetWorldLocation (Variables|/Script/OValTan.OValTanCharacter|GetFirstPersonCameraComponent _asbp_genji_2)) (+ (Transformation|GetWorldLocation (Variables|/Script/OValTan.OValTanCharacter|GetFirstPersonCameraComponent _asbp_genji_2)) (* (Math|Vector|GetForwardVector (Variables|/Script/OValTan.OValTanCharacter|GetFirstPersonCameraComponent _asbp_genji_2)) (Variables|Default|Getlength))) "TraceTypeQuery1" false 0 "Persistent"))
  (Variables|Default|SetPyochanglocation (.TraceEnd (Collision|BreakHitResult _outhit)))
  (Variables|Default|Setstartlocation (Transformation|GetActorLocation))
  (CallFunction|DashMovement)
  (Actor|SetOwner _asbp_genji_2))

(event Collision|EventActorBeginOverlap
  (params (OtherActor :type Actor%20Object%20Reference)))

(event EventTick
  (params (DeltaSeconds :type Float%20%28single-precision%29)))

(fn ConstructionScript)