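; NBP_Slash_3 is a slash actor that follows the first-person camera of its owning BP_Genji2 character.
; On BeginPlay it casts its owner to BP_Genji2 and stores the reference.
; Every Tick it moves to SlashLength units along the camera's forward vector and rotates to face that direction, without sweeping.
; It contains no overlap or damage logic.
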(event EventBeginPlay
  (bind _asbp_genji_2 (Utilities|Casting|CastToBP_Genji2 (Components|GetOwner)))
  (Variables|Default|SetAs%20BP%20Genji%202 _asbp_genji_2))

(event Collision|EventActorBeginOverlap
  (params (OtherActor :type Actor%20Object%20Reference)))

(event EventTick
  (params (DeltaSeconds :type Float%20%28single-precision%29))
  (bind _as_bp_genji_2 (Variables|Default|GetAs%20BP%20Genji%202))
  (bind _firstpersoncameracomponent (Variables|/Script/OValTan.OValTanCharacter|GetFirstPersonCameraComponent _as_bp_genji_2))
  (bind _returnvalue (Math|Vector|GetForwardVector _firstpersoncameracomponent))
  (Transformation|SetActorLocation (+ (Transformation|GetWorldLocation _firstpersoncameracomponent) (* _returnvalue (Variables|/Game/JJH/blueprint/BP_Genji2.BP_Genji2_C|Getslash%20length _as_bp_genji_2))) false false)
  (Transformation|SetActorRotation (Math|Conversions|RotationFromXVector _returnvalue)))

(fn ConstructionScript)