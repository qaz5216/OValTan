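; BP_Pyochang is a thrown projectile for the Genji character that deals fixed damage to actors overlapping its sphere.
; On BeginPlay it line-traces from player 0's first-person camera with persistent debug drawing.
; It targets the trace's end point, not the hit location.
; A Timeline then lerps the actor from spawn point to target with a swept move, rather than using projectile movement.
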(event OnComponentBeginOverlap(Sphere)
  (params (OverlappedComponent :type Primitive%20Component%20Object%20Reference) (OtherActor :type Actor%20Object%20Reference) (OtherComp :type Primitive%20Component%20Object%20Reference) (OtherBodyIndex :type Integer) (bFromSweep :type Boolean) (SweepResult :type Hit%20Result%20Structure%20%28by%20ref%29))
  (Game|Damage|ApplyDamage OtherActor 24.0 0 0))

(event Custom|DashMovement
  (bind _alpha (Timeline|Timeline PlayFromStart)
    (:Update
      (Transformation|SetActorLocation (Math|Vector|Lerp(Vector) (Variables|Default|Getstartlocation) (Variables|Default|GetPyochanglocation) _alpha) true false))))

(event EventBeginPlay
  (bind _asbp_gen_ji (Utilities|Casting|CastToBP_GenJi (Game|GetPlayerCharacter 0)))
  (bind _outhit (Collision|LineTraceByChannel (Transformation|GetWorldLocation (Variables|/Game/JJH/blueprint/BP_GenJi.BP_GenJi_C|GetFirstPersonCamera _asbp_gen_ji)) (+ (Transformation|GetWorldLocation (Variables|/Game/JJH/blueprint/BP_GenJi.BP_GenJi_C|GetFirstPersonCamera _asbp_gen_ji)) (* (Math|Vector|GetForwardVector (Variables|/Game/JJH/blueprint/BP_GenJi.BP_GenJi_C|GetFirstPersonCamera _asbp_gen_ji)) (Variables|Default|Getlength))) "TraceTypeQuery1" false 0 "Persistent"))
  (Variables|Default|SetPyochanglocation (.TraceEnd (Collision|BreakHitResult _outhit)))
  (Variables|Default|Setstartlocation (Transformation|GetActorLocation))
  (CallFunction|DashMovement))

(event Collision|EventActorBeginOverlap
  (params (OtherActor :type Actor%20Object%20Reference)))

(event EventTick
  (params (DeltaSeconds :type Float%20%28single-precision%29)))

(fn ConstructionScript)