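; Shuriken (pyochang) projectile for BP_Genji2 that damages OValTanCharacters it overlaps.
; On spawn it line-traces forward and a Timeline lerps it with sweep to the trace end point, ignoring any hit, with timed self-destruction.
; Sphere overlaps skip the owner by display name, then apply fixed damage, charge player 0's ultimate gauge and update hit, headshot and server-only kill feedback.
; Headshots are detected by component name and add no damage.
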(event OnComponentBeginOverlap(Sphere)
  (params (OverlappedComponent :type Primitive%20Component%20Object%20Reference) (OtherActor :type Actor%20Object%20Reference) (OtherComp :type Primitive%20Component%20Object%20Reference) (OtherBodyIndex :type Integer) (bFromSweep :type Boolean) (SweepResult :type Hit%20Result%20Structure%20%28by%20ref%29))
  (bind _asoval_tan_character (Utilities|Casting|CastToOValTanCharacter OtherActor))
  (if (not (Utilities|Enum|Equal(Enum) (Utilities|GetDisplayName (Components|GetOwner)) (Utilities|GetDisplayName _asoval_tan_character)))
    (if (not (Utilities|String|Contains (Utilities|GetObjectName _asoval_tan_character) "Head"))
      (CallFunction|CustomEvent))))

(event Custom|DashMovement
  (bind _alpha (Timeline|Timeline PlayFromStart)
    (:Update
      (Transformation|SetActorLocation (Math|Vector|Lerp(Vector) (Variables|Default|Getstartlocation) (Variables|Default|GetPyochanglocation) _alpha) true false))))

(event Custom|CustomEvent
  (Game|Damage|ApplyDamage (stale OnComponentBeginOverlap(Sphere) OtherActor) 27.0 0 0)
  (if (> (+ (Variables|/Script/OValTan.OValTanCharacter|GetGauge_Ultimate_Cur (stale Custom|CustomEvent_0 _asbp_genji_2)) 2.7) 1e+02)
    (Variables|/Script/OValTan.OValTanCharacter|SetGauge_Ultimate_Cur (stale Custom|CustomEvent_0 _asbp_genji_2) 1e+02)
    (else
      (Variables|/Script/OValTan.OValTanCharacter|SetGauge_Ultimate_Cur (stale Custom|CustomEvent_0 _asbp_genji_2) (+ (Variables|/Script/OValTan.OValTanCharacter|GetGauge_Ultimate_Cur (stale Custom|CustomEvent_0 _asbp_genji_2)) 2.7))))
  (bind _asbp_uibase (Utilities|Casting|CastToBP_UIBase (Variables|/Script/OValTan.OValTanCharacter|GetIngame_UI (stale Custom|CustomEvent_0 _asbp_genji_2))))
  (Default|SetCURUlt _asbp_uibase)
  (Default|PlayAttack _asbp_uibase)
  (if (Utilities|String|Contains (Utilities|GetObjectName (stale OnComponentBeginOverlap(Sphere) OtherComp)) "Head")
    (Default|AttackHead _asbp_uibase))
  (bind _asoval_tan_character (Utilities|Casting|CastToOValTanCharacter (stale OnComponentBeginOverlap(Sphere) OtherActor)))
  (if (<= (Variables|/Script/OValTan.OValTanCharacter|GetHP_Cur _asoval_tan_character) 0)
    (if (Networking|IsServer)
      (Class|OValTanCharacter|Killing (stale Custom|CustomEvent_0 _asbp_genji_2))
      (Default|PlayKilling _asbp_uibase)
      (Utilities|FlowControl|Delay 0.2)
      (Actor|DestroyActor :!label _label))
    (else
      (Utilities|FlowControl|Delay 0.2)
      (goto _label))))

(event Custom|CustomEvent_0
  (bind _returnvalue (Transformation|GetActorLocation))
  (bind _asbp_genji_2 (Utilities|Casting|CastToBP_Genji2 (Game|GetPlayerCharacter 0)))
  (bind _outhit (Collision|LineTraceByChannel (+ _returnvalue (* (Transformation|GetActorForwardVector) (Variables|Default|Getlengthstart))) (+ _returnvalue (* (Transformation|GetActorForwardVector) (Variables|Default|Getlength))) "TraceTypeQuery1" false 0 "None"))
  (Variables|Default|SetPyochanglocation (.TraceEnd (Collision|BreakHitResult _outhit)))
  (Variables|Default|Setstartlocation (Transformation|GetActorLocation))
  (CallFunction|DashMovement)
  (Utilities|FlowControl|Delay 0.2)
  (Utilities|FlowControl|Delay 4.8)
  (Actor|DestroyActor))

(event EventBeginPlay
  (CallFunction|CustomEvent0))

(event Collision|EventActorBeginOverlap
  (params (OtherActor :type Actor%20Object%20Reference)))

(event EventTick
  (params (DeltaSeconds :type Float%20%28single-precision%29)))

(fn ConstructionScript)

(fn OnRepLength)

(fn OnRepPyochanglocation)

(fn OnRepStartlocation)

(fn OnRepSpawnController)

(fn OnRepDamage)