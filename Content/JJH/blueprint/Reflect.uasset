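; Genji's deflect actor, which follows the owning BP_Genji2's first-person camera to send attacks back.
; Overlaps destroy the other actor and, like received damage, feed a Damage-based branch.
; That branch spawns a shuriken below 20 damage, otherwise line-traces damage; its pulse-bomb case is unreachable behind that check.
; A separate TracerReflect event plays melee montages and sound, briefly spawns a TracerReflect actor and applies line-trace damage.
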(event OnComponentBeginOverlap(ReflectColli)
  (params (OverlappedComponent :type Primitive%20Component%20Object%20Reference) (OtherActor :type Actor%20Object%20Reference) (OtherComp :type Primitive%20Component%20Object%20Reference) (OtherBodyIndex :type Integer) (bFromSweep :type Boolean) (SweepResult :type Hit%20Result%20Structure%20%28by%20ref%29))
  (bind _as_bp_genji_2 (Variables|Default|GetAs%20BP%20Genji%202))
  (bind _as_bp_genji_2_2 (Variables|Default|GetAs%20BP%20Genji%202))
  (bind _as_bp_genji_2_3 (Variables|Default|GetAs%20BP%20Genji%202))
  (bind _firstpersoncameracomponent (Variables|/Script/OValTan.OValTanCharacter|GetFirstPersonCameraComponent _as_bp_genji_2))
  (bind _firstpersoncameracomponent_2 (Variables|/Script/OValTan.OValTanCharacter|GetFirstPersonCameraComponent _as_bp_genji_2_3))
  (bind _returnvalue (Transformation|GetWorldLocation _firstpersoncameracomponent))
  (bind _returnvalue_2 (Math|Vector|GetForwardVector _firstpersoncameracomponent_2))
  (Actor|DestroyActor OtherActor)
  (Utilities|IsValid OtherActor
    (:Is%20Valid
      (Actor|DestroyActor)
      (Utilities|IsValid OtherActor
        (:Is%20Valid
          (Actor|DestroyActor)
          (Animation|Montage|PlayMontage (Variables|/Script/OValTan.OValTanCharacter|GetMesh3P _as_bp_genji_2_2) "/Game/JJH/Animation/G_Melee_Montage.G_Melee_Montage"
            (:then
              (Animation|Montage|PlayMontage (Variables|/Script/OValTan.OValTanCharacter|GetMesh1P _as_bp_genji_2_2) "/Game/JJH/Animation/MeleeAttack.MeleeAttack"
                (:then
                  _)))))
        (:Is%20Not%20Valid
          _)))
    (:Is%20Not%20Valid
      _))
  (Audio|PlaySound2D "/Game/SFX/SFX_Genji/SFX_G_Ref_Success_1_Cue.SFX_G_Ref_Success_1_Cue" 1.0 1.0 0.0 0 0)
  (if (< (stale Game|Damage|EventAnyDamage Damage) 2e+01)
    (Game|SpawnActorfromClass "/Game/JJH/blueprint/BP_Pyochang_8.BP_Pyochang_8_C" (Math|Transform|MakeTransform (+ (Transformation|GetWorldLocation _firstpersoncameracomponent_2) (* _returnvalue_2 (Variables|Default|Getreflectstart))) (Math|Conversions|RotationFromXVector _returnvalue_2) "1.000000,1.000000,1.000000") "Undefined" "MultiplyWithRoot" self 0)
    (elif (== (stale Game|Damage|EventAnyDamage Damage) 2.0)
      (bind _returnvalue_3 (Game|SpawnActorfromClass "/Game/SYH/BP_TracerPulseBomb.BP_TracerPulseBomb_C" (Math|Transform|MakeTransform (Transformation|GetWorldLocation (Variables|Default|GetHalf_Circle)) (Transformation|GetActorRotation) "1.000000,1.000000,1.000000") "Undefined" "MultiplyWithRoot" 0 0))
      (Physics|SetPhysicsLinearVelocity (Variables|/Game/SYH/BP_TracerPulseBomb.BP_TracerPulseBomb_C|GetSphere _returnvalue_3) (* (Math|Vector|GetUnitDirection(Vector) (Transformation|GetActorLocation) (Transformation|GetActorLocation _returnvalue_3)) (Variables|Default|GetSpeed)) true "None")
      (else
        (bind _outhit (Collision|LineTraceByChannel (+ _returnvalue (* (Math|Vector|GetForwardVector _firstpersoncameracomponent) (Variables|Default|Getreflectstart))) (+ _returnvalue (* (Math|Vector|GetForwardVector _firstpersoncameracomponent) (Variables|Default|GetReflectend))) "TraceTypeQuery1" false 0 "Persistent"))
        (Game|Damage|ApplyDamage (.HitActor (Collision|BreakHitResult _outhit)) 5.0 0 0)))))

(event Custom|TracerReflect
  (bind _reflectstart (Variables|Default|Getreflectstart))
  (bind _as_bp_genji_2 (Variables|Default|GetAs%20BP%20Genji%202))
  (bind _as_bp_genji_2_2 (Variables|Default|GetAs%20BP%20Genji%202))
  (bind _firstpersoncameracomponent (Variables|/Script/OValTan.OValTanCharacter|GetFirstPersonCameraComponent _as_bp_genji_2_2))
  (bind _returnvalue (Transformation|GetWorldLocation _firstpersoncameracomponent))
  (bind _returnvalue_2 (Math|Vector|GetForwardVector _firstpersoncameracomponent))
  (bind _returnvalue_3 (* _returnvalue_2 _reflectstart))
  (bind _returnvalue_4 (+ _returnvalue _returnvalue_3))
  (Animation|Montage|PlayMontage (Variables|/Script/OValTan.OValTanCharacter|GetMesh3P _as_bp_genji_2) "/Game/CYS/CYS_Genji/G_Anim/G_L_Melee_Montage.G_L_Melee_Montage"
    (:then
      (Animation|Montage|PlayMontage (Variables|/Script/OValTan.OValTanCharacter|GetMesh1P _as_bp_genji_2) "/Game/JJH/Animation/MeleeAttack.MeleeAttack"
        (:then
          (Audio|PlaySound2D "/Game/SFX/SFX_Genji/SFX_G_Ref_Success_1_Cue.SFX_G_Ref_Success_1_Cue" 1.0 1.0 0.0 0 0)
          (Utilities|FlowControl|Sequence
            (:then_0
              (if (not (Variables|Default|Getisreflecting))
                (Variables|Default|Setisreflecting true)
                (bind _returnvalue_5 (Game|SpawnActorfromClass "/Game/JJH/blueprint/TracerReflect.TracerReflect_C" (Math|Transform|MakeTransform _returnvalue_4 (Transformation|GetActorRotation) "1.000000,1.000000,1.000000") "Undefined" "MultiplyWithRoot" 0 0))
                (Utilities|FlowControl|Delay 0.05)
                (Actor|DestroyActor _returnvalue_5)
                (Variables|Default|Setisreflecting false)))
            (:then_1
              (bind _outhit (Collision|LineTraceByChannel _returnvalue_4 (+ _returnvalue (* (Math|Vector|GetForwardVector _firstpersoncameracomponent) (Variables|Default|GetReflectend))) "TraceTypeQuery3" false 0 "Persistent"))
              (Game|Damage|ApplyDamage (.HitActor (Collision|BreakHitResult _outhit)) 3.0 0 0))))))))

(event EventBeginPlay
  (bind _asbp_genji_2 (Utilities|Casting|CastToBP_Genji2 (Components|GetOwner)))
  (Variables|Default|SetAs%20BP%20Genji%202 _asbp_genji_2))

(event Collision|EventActorBeginOverlap
  (params (OtherActor :type Actor%20Object%20Reference)))

(event EventTick
  (params (DeltaSeconds :type Float%20%28single-precision%29))
  (bind _as_bp_genji_2 (Variables|Default|GetAs%20BP%20Genji%202))
  (bind _firstpersoncameracomponent (Variables|/Script/OValTan.OValTanCharacter|GetFirstPersonCameraComponent _as_bp_genji_2))
  (bind _returnvalue (Math|Vector|GetForwardVector _firstpersoncameracomponent))
  (Transformation|SetActorLocation (+ (Transformation|GetWorldLocation _firstpersoncameracomponent) (* _returnvalue (Variables|/Game/JJH/blueprint/BP_Genji2.BP_Genji2_C|Getreflect%20damage _as_bp_genji_2))) false false)
  (Transformation|SetActorRotation (Math|Conversions|RotationFromXVector _returnvalue)))

(event Game|Damage|EventAnyDamage
  (params (Damage :type Float%20%28single-precision%29) (DamageType :type Damage%20Type%20Object%20Reference) (InstigatedBy :type Controller%20Object%20Reference) (DamageCauser :type Actor%20Object%20Reference))
  (bind _as_bp_genji_2 (Variables|Default|GetAs%20BP%20Genji%202))
  (bind _as_bp_genji_2_2 (Variables|Default|GetAs%20BP%20Genji%202))
  (bind _firstpersoncameracomponent (Variables|/Script/OValTan.OValTanCharacter|GetFirstPersonCameraComponent _as_bp_genji_2))
  (bind _firstpersoncameracomponent_2 (Variables|/Script/OValTan.OValTanCharacter|GetFirstPersonCameraComponent _as_bp_genji_2_2))
  (bind _returnvalue (Transformation|GetWorldLocation _firstpersoncameracomponent))
  (bind _returnvalue_2 (Math|Vector|GetForwardVector _firstpersoncameracomponent_2))
  (if (< Damage 2e+01)
    (Game|SpawnActorfromClass "/Game/JJH/blueprint/BP_Pyochang_8.BP_Pyochang_8_C" (Math|Transform|MakeTransform (+ (Transformation|GetWorldLocation _firstpersoncameracomponent_2) (* _returnvalue_2 (Variables|Default|Getreflectstart))) (Math|Conversions|RotationFromXVector _returnvalue_2) "1.000000,1.000000,1.000000") "Undefined" "MultiplyWithRoot" self 0)
    (elif (== Damage 2.0)
      (bind _returnvalue_3 (Game|SpawnActorfromClass "/Game/SYH/BP_TracerPulseBomb.BP_TracerPulseBomb_C" (Math|Transform|MakeTransform (Transformation|GetWorldLocation (Variables|Default|GetHalf_Circle)) (Transformation|GetActorRotation) "1.000000,1.000000,1.000000") "Undefined" "MultiplyWithRoot" 0 0))
      (Physics|SetPhysicsLinearVelocity (Variables|/Game/SYH/BP_TracerPulseBomb.BP_TracerPulseBomb_C|GetSphere _returnvalue_3) (* (Math|Vector|GetUnitDirection(Vector) (Transformation|GetActorLocation) (Transformation|GetActorLocation _returnvalue_3)) (Variables|Default|GetSpeed)) true "None")
      (else
        (bind _outhit (Collision|LineTraceByChannel (+ _returnvalue (* (Math|Vector|GetForwardVector _firstpersoncameracomponent) (Variables|Default|Getreflectstart))) (+ _returnvalue (* (Math|Vector|GetForwardVector _firstpersoncameracomponent) (Variables|Default|GetReflectend))) "TraceTypeQuery1" false 0 "Persistent"))
        (Game|Damage|ApplyDamage (.HitActor (Collision|BreakHitResult _outhit)) 5.0 0 0)))))

(fn ConstructionScript)

(fn NewFunction
  (params (NewParam :type Boolean) (NewParam1 :type Boolean))
  (return false))