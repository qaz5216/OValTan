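; BP_TracerPulseBomb is Tracer's pulse bomb actor, which attaches to any actor its mesh overlaps and detonates.
; BeginPlay waits briefly, plays a timer sound and calls PulseBombGO regardless of contact, while each overlap also schedules it on a timer.
; PulseBombGO spawns the effect actor, plays the blast sound, hides the mesh and destroys the bomb after a delay.
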(event OnComponentBeginOverlap(PulsebombMesh)
  (params (OverlappedComponent :type Primitive%20Component%20Object%20Reference) (OtherActor :type Actor%20Object%20Reference) (OtherComp :type Primitive%20Component%20Object%20Reference) (OtherBodyIndex :type Integer) (bFromSweep :type Boolean) (SweepResult :type Hit%20Result%20Structure%20%28by%20ref%29))
  (Transformation|AttachActorToActor OtherActor "None" "KeepWorld" "KeepRelative" "KeepWorld" true)
  (Utilities|FlowControl|Sequence
    (:then_1
      (Utilities|Time|SetTimerbyEvent (delegate Custom|PulseBombGO) 2.0))))

(event Custom|PulseBombGO
  (Game|SpawnActorfromClass "/Game/SYH/BP_PulseBombEFFECT.BP_PulseBombEFFECT_C" (Math|Transform|MakeTransform (Transformation|GetActorLocation) "0, 0, 0" "1.000000,1.000000,1.000000") "Undefined" "MultiplyWithRoot" 0 0)
  (Audio|PlaySoundatLocation (Variables|Default|GetPulseBombSound) (Transformation|GetActorLocation) "0, 0, 0" 1.0 1.0 0.0 0 0 0 0)
  (Development|SetHiddeninGame (Variables|Default|GetPulsebombMesh) true false)
  (Utilities|FlowControl|Delay 2.0)
  (Actor|DestroyActor))

(event EventBeginPlay
  (Utilities|FlowControl|Delay 1.0)
  (Audio|PlaySoundatLocation (Variables|Default|GetPulseBomb_TimerSound) (Transformation|GetActorLocation) "0, 0, 0" 1.0 1.0 0.0 0 0 0 0)
  (CallFunction|PulseBombGO))

(event EventTick
  (params (DeltaSeconds :type Float%20%28single-precision%29)))

(fn ConstructionScript)