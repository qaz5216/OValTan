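; Tracer Blueprint that handles attack, reload and ultimate inputs and drives the in-game HUD, apparently as test wiring.
; BeginPlay creates the BP_UIBase widget and adds it to the viewport.
; Attack decrements ammo without a bounds check and prints a debug string, while reload only calls the ammo display update.
; Ultimate input raises the gauge in small steps, resets it past the cap, then updates the HUD.
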(event Input|EnhancedActionEvents|EnhancedInputActionIA_Attack1
  (params (ActionValue :type Boolean) (ElapsedSeconds :type Float%20%28double-precision%29) (TriggeredSeconds :type Float%20%28double-precision%29) (InputAction :type Input%20Action%20Object%20Reference :default "/Game/FirstPerson/Input/Actions/IA_Attack1.IA_Attack1"))
  (:Triggered
    (Variables|Default|SetAmmo_Cur (- (Variables|Default|GetAmmo_Cur) 1))
    (Default|SetCurAmmo (Variables|Default|GetIngameUI))
    (Development|PrintString "Hello")))

(event Input|EnhancedActionEvents|EnhancedInputActionIA_Reload
  (params (ActionValue :type Boolean) (ElapsedSeconds :type Float%20%28double-precision%29) (TriggeredSeconds :type Float%20%28double-precision%29) (InputAction :type Input%20Action%20Object%20Reference :default "/Game/FirstPerson/Input/Actions/IA_Reload.IA_Reload"))
  (:Triggered
    (Default|SetCurAmmo (Variables|Default|GetIngameUI))))

(event Input|EnhancedActionEvents|EnhancedInputActionIA_Ultimate
  (params (ActionValue :type Boolean) (ElapsedSeconds :type Float%20%28double-precision%29) (TriggeredSeconds :type Float%20%28double-precision%29) (InputAction :type Input%20Action%20Object%20Reference :default "/Game/FirstPerson/Input/Actions/IA_Ultimate.IA_Ultimate"))
  (:Triggered
    (if (> (+ (Variables|Default|GetGauge_Ultimate_Cur) 2.0) 1e+02)
      (Variables|Default|SetGauge_Ultimate_Cur 0.0)
      (else
        (Variables|Default|SetGauge_Ultimate_Cur (+ (Variables|Default|GetGauge_Ultimate_Cur) 2.0))))
    (Default|SetCURUlt (Variables|Default|GetIngameUI))))

(event EventTick
  (params (DeltaSeconds :type Float%20%28single-precision%29)))

(event Collision|EventActorBeginOverlap
  (params (OtherActor :type Actor%20Object%20Reference)))

(event EventBeginPlay
  (bind _returnvalue (UserInterface|CreateWidget "/Game/PKM/UI_Base/BP_UIBase.BP_UIBase_C"))
  (bind _output_get (Variables|Default|SetIngameUI _returnvalue))
  (UserInterface|Viewport|AddtoViewport _output_get 0))

(fn ConstructionScript)